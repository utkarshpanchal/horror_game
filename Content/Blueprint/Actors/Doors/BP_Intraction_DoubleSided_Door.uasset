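; Interactable double-sided door actor that swings open away from the player and closes again on the next interaction.
; On Interact, a closed door takes the dot product of its forward vector and the player-to-door direction to pick the swing side.
; A timeline lerps the mesh's relative yaw to a right angle on that side, then plays in reverse to close it.
; PlayerRef is read but never assigned in these graphs.
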(event EventBeginPlay
  (|CallParentFunction) ; This node is disabled and will not be called.\nDrag off pins to build functionality.
)

(event Collision|EventActorBeginOverlap
  (params (OtherActor :type Actor%20Object%20Reference))
  (|CallParentFunction OtherActor) ; This node is disabled and will not be called.\nDrag off pins to build functionality.
)

(event EventTick
  (params (DeltaSeconds :type Float%20%28single-precision%29))
  (|CallParentFunction DeltaSeconds) ; This node is disabled and will not be called.\nDrag off pins to build functionality.
)

(event EventInteract
  (bind _self self)
  (if (Variables|Default|GetisDoorClose)
    (Variables|Default|SetisDoorClose false)
    (Variables|Default|SetDot%20Prouduct (Math|Vector|DotProduct (Math|Vector|Normalize (- (Transformation|GetActorLocation _self) (Transformation|GetActorLocation (Variables|Default|GetPlayerRef)))) (Transformation|GetActorForwardVector _self)))
    (bind _alpha (Timeline|ToggleOpenCloseDoor PlayFromStart)
      (:Update
        (Transformation|SetRelativeRotation (Variables|Default|GetDoorMesh) (Math|Rotator|MakeRotator 0.0 0.0 (Math|Float|Lerp 0.0 (select (>= (Variables|Default|GetDot%20Prouduct) 0.0) 9e+01 -9e+01) _alpha)) false false)))
    (else
      (Variables|Default|SetisDoorClose true)
      (Timeline|ToggleOpenCloseDoor ReverseFromEnd))))

(fn ConstructionScript
  (|CallParentFunction))