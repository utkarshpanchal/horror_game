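; Movement component that gives a character sprinting limited by stamina, switching max walk speed between walk and sprint values.
; Initialize stores the character reference, and sprinting starts only when stamina remains and the character is moving.
; Looping timers drain stamina until it empties or movement stops, then refill it after a retriggerable delay following sprint end.
; Both timer events print stamina to screen for debugging.
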(event Custom|StartSprinting
  (if (and (> (Variables|Default|GetCurrent_stamina) (Variables|Default|GetMin_stamina)) (> (Math|Vector|VectorLength (Transformation|GetVelocity (Variables|Default|GetPlayerRef))) 1e+01))
    (Utilities|Time|ClearTimerbyFunctionName 0 "RegenerateStamina")
    (CallFunction|SetPlayerMaxWalkSpeed (Variables|Default|GetSprint_speed))
    (Utilities|Time|SetTimerbyFunctionName 0 "SprintTimer" 0.1 true)))

(event Custom|SprintTimer
  (if (> (Math|Vector|VectorLength (Transformation|GetVelocity (Variables|Default|GetPlayerRef))) 1e+01)
    (Development|PrintString (Utilities|String|ToString(Float) (Variables|Default|GetCurrent_stamina)) true true "(R=1.000000,G=0.000000,B=0.012675,A=1.000000)")
    (Variables|Default|SetCurrent_stamina (Math|Float|Clamp(Float) (- (Variables|Default|GetCurrent_stamina) 1.0) (Variables|Default|GetMin_stamina) (Variables|Default|GetMax_stamina)))
    (if (<= (Variables|Default|GetCurrent_stamina) (Variables|Default|GetMin_stamina))
      (CallFunction|StopSprint))
    (else
      (CallFunction|StopSprint))))

(event Custom|StopSprint
  (Utilities|Time|ClearTimerbyFunctionName 0 "SprintTimer")
  (CallFunction|SetPlayerMaxWalkSpeed (Variables|Default|GetWalk_speed))
  (Utilities|FlowControl|RetriggerableDelay 5.0)
  (if (not (Class|KismetSystemLibrary|IsTimerActive 0 "SprintTimer"))
    (Utilities|Time|SetTimerbyFunctionName 0 "RegenerateStamina" 0.03 true)))

(event Custom|RegenerateStamina
  (Variables|Default|SetCurrent_stamina (Math|Float|Clamp(Float) (+ (Variables|Default|GetCurrent_stamina) 1.0) (Variables|Default|GetMin_stamina) (Variables|Default|GetMax_stamina)))
  (Development|PrintString (Utilities|String|ToString(Float) (Variables|Default|GetCurrent_stamina)))
  (if (>= (Variables|Default|GetCurrent_stamina) (Variables|Default|GetMax_stamina))
    (Utilities|Time|ClearTimerbyFunctionName 0 "RegenerateStamina")))

(fn Initialize
  (params (Character :type Character%20Object%20Reference))
  (Variables|Default|SetPlayerRef Character)
  (Variables|/Script/Engine.CharacterMovementComponent|SetMaxWalkSpeed (Variables|/Script/Engine.Character|GetCharacterMovement (Variables|Default|GetPlayerRef)) (Variables|Default|GetWalk_speed)))

(fn SetPlayerMaxWalkSpeed
  (params (MaxWalkSpeed :type Float%20%28single-precision%29))
  (Variables|/Script/Engine.CharacterMovementComponent|SetMaxWalkSpeed (Variables|/Script/Engine.Character|GetCharacterMovement (Variables|Default|GetPlayerRef)) MaxWalkSpeed))